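; Player controller that turns mouse, device tilt and touch input into camera yaw and pitch, each scaled by its own sensitivity.
; Mouse axes and tilt apply only while the current device is Mouse; first-finger touch drags apply regardless of device.
; Tilt and touch work on deltas from the last stored value, with touch dividing by sensitivity rather than multiplying.
; Getter and setter functions expose the current device and per-device sensitivities.
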(event `InputAxis|MouseY`
  (params (AxisValue :type "Float (single-precision)"))
  (if (`|EnumEquality` (`self.CurrentControllingDevice`) "NewEnumerator0")
    (`self.AddPitchInput` (* AxisValue (`self.MouseSensitivityCurrent`)))))

(event `InputAxis|MouseX`
  (params (AxisValue :type "Float (single-precision)"))
  (if (`|EnumEquality` (`self.CurrentControllingDevice`) "NewEnumerator0")
    (`self.AddYawInput` (* AxisValue (`self.MouseSensitivityCurrent`)))))

(event `InputVectorAxis|Tilt`
  (params (AxisValue :type "Vector Structure"))
  (bind _returnvalue (* AxisValue (`self.GyroSensitivityCurrent`)))
  (if (`|EnumEquality` (`self.CurrentControllingDevice`) "NewEnumerator0")
    (`self.AddYawInput` (* (.x (- _returnvalue (`self.LastTilt`))) -1.0))
    (`self.AddPitchInput` (.z (- _returnvalue (`self.LastTilt`))))
    (set `self.LastTilt` _returnvalue)))

(event `InputTouch`
  (params (Location :type "Vector Structure") (FingerIndex :type "ETouchIndex Enum"))
  (bind (_lasttouch_x _lasttouch_y) (`KismetMathLibrary.BreakVector` (`self.LastTouch`)))
  (:`Pressed`
    (if (== FingerIndex 0)
      (set `self.LastTouch` Location)))
  (:`Moved`
    (if (== FingerIndex 0)
      (`self.AddYawInput` (/ (- (.x Location) _lasttouch_x) (`self.TouchSensitivityCurrent`)))
      (`self.AddPitchInput` (/ (- (.z Location) _lasttouch_y) (`self.TouchSensitivityCurrent`)))
      (set `self.LastTouch` Location))))

(fn `GetCurrentContollingDevice`
  (returns (CurrentCotrollingDevice :type "/Game/Shimeji/BluePrints/BP_EnumControllingDevice Enum"))
  (return (`self.CurrentControllingDevice`)))

(fn `GetSensitivity`
  (params (WhichDevice :type "/Game/Shimeji/BluePrints/BP_EnumControllingDevice Enum" :default "NewEnumerator0") (CurrentDevice :type Boolean))
  (returns (Sensitivity :type "Float (double-precision)"))
  (locals (LocalSensitivity :type "Float (double-precision)"))
  (`|ExecutionSequence`
    (:`then_0`
      (if CurrentDevice
        (switch `/Game/Shimeji/BluePrints/BP_EnumControllingDevice` (`self.CurrentControllingDevice`)
          (:`NewEnumerator0`
            (set `local.LocalSensitivity` (`self.MouseSensitivityCurrent`)))
          (:`NewEnumerator1`
            (set `local.LocalSensitivity` (`self.TouchSensitivityCurrent`)))
          (:`NewEnumerator2`
            (set `local.LocalSensitivity` (`self.GyroSensitivityCurrent`))))
        (else
          (switch `/Game/Shimeji/BluePrints/BP_EnumControllingDevice` WhichDevice
            (:`NewEnumerator0`
              (set `local.LocalSensitivity` (`self.MouseSensitivityCurrent`)))
            (:`NewEnumerator1`
              (set `local.LocalSensitivity` (`self.TouchSensitivityCurrent`)))
            (:`NewEnumerator2`
              (set `local.LocalSensitivity` (`self.GyroSensitivityCurrent`)))))))
    (:`then_1`
      (return (`local.LocalSensitivity`)))))

(fn `SetCurrentControllingDevice`
  (params (NewControllingDevie :type "/Game/Shimeji/BluePrints/BP_EnumControllingDevice Enum" :default "NewEnumerator0"))
  (set `self.CurrentControllingDevice` NewControllingDevie))

(fn `SetSensitivity`
  (params (WhichDevice :type "/Game/Shimeji/BluePrints/BP_EnumControllingDevice Enum" :default "NewEnumerator0") (NewSensitivity :type "Float (double-precision)"))
  (switch `/Game/Shimeji/BluePrints/BP_EnumControllingDevice` WhichDevice
    (:`NewEnumerator0`
      (set `self.MouseSensitivityCurrent` NewSensitivity))
    (:`NewEnumerator1`
      (set `self.TouchSensitivityCurrent` NewSensitivity))
    (:`NewEnumerator2`
      (set `self.GyroSensitivityCurrent` NewSensitivity))))

(fn `UserConstructionScript`)